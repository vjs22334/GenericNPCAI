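; BP_CoverGoalGenerator is a Utility AI goal generator that maintains a cover goal for a ShooterBaseCharacter.
; Initialize stores the owning character and goal generator component, and the first EvaluateGoal creates a BP_CoverGoalData and registers it with that component.
; While that data is valid, later evaluations run the EQS_Cover query in random-best-25% mode.
; The finish callback writes the first result into the goal's location without checking query status.
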(event `CustomEvent`
  (params (QueryInstance :type "EnvQueryInstanceBlueprintWrapper Object Reference") (QueryStatus :type "EEnvQueryStatus Enum" :default "Processing"))
  (bind _resultlocations (`EnvQueryInstanceBlueprintWrapper.GetQueryResultsAsLocations` QueryInstance))
  (set `/Game/MyContent/AI/UtilityAI/GoalGenerators/BP_CoverGoalData.Location` (`|GetArrayItem` _resultlocations) (`self.Generated Goal Data`)))

(event `self.EvaluateGoal`
  (params (goalOwner :type "Actor Object Reference") (DeltaTime :type "Float (single-precision)"))
  (if (`KismetSystemLibrary.IsValid` (`self.Generated Goal Data`))
    (bind _returnvalue (`EnvQueryManager.RunEQSQuery` "/Game/MyContent/EQS/EQS_Cover.EQS_Cover" (`self.Goal Owner`) "RandomBest25Pct"))
    (add `EnvQueryInstanceBlueprintWrapper.OnQueryFinishedEvent` _returnvalue (delegate `CustomEvent`))
    (else
      (bind _returnvalue_2 (`|GenericCreateObject` "/Game/MyContent/AI/UtilityAI/GoalGenerators/BP_CoverGoalData.BP_CoverGoalData_C"))
      (set `self.Location` (0.0 0.0 0.0))
      (`GoalGeneratorComponent.AddGoal` (`self.Goal Generator Component`) _returnvalue_2)
      (set `self.Generated Goal Data` _returnvalue_2))))

(event `self.Initialize`
  (params (goalOwner :type "Actor Object Reference") (owner :type "GoalGeneratorComponent Object Reference"))
  (bind _asshooter_base_character (cast `ShooterBaseCharacter` goalOwner))
  (set `self.Goal Owner` _asshooter_base_character)
  (set `self.Goal Generator Component` owner))