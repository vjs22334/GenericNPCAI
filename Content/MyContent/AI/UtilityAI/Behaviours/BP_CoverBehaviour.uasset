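; Utility AI behaviour that moves a shooter character to a cover location.
; On enter it stores the cover goal data and marks itself running and non-interruptible.
; Each tick it issues an AI MoveTo from the owning character to that location with a tight acceptance radius, without handling the move result.
; Its selection score is a constant, regardless of the goal data.
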(event `self.BehaviourEnter`
  (params (GoalData :type "BaseGoalData Object Reference"))
  (bind _asbp_cover_goal_data (cast `/Game/MyContent/AI/UtilityAI/GoalGenerators/BP_CoverGoalData` GoalData))
  (set `self.Cover Goal Data` _asbp_cover_goal_data)
  (set `self.M_BehaviourInterruptibilityState` "NOTINTERRUPTIBLE")
  (set `self.M_BehaviourState` "RUNNING"))

(event `self.BehaviourTick`
  (params (DeltaTime :type "Float (single-precision)"))
  (`|AIMoveTo` (`self.Owner Actor`) (`/Game/MyContent/AI/UtilityAI/GoalGenerators/BP_CoverGoalData.Location` (`self.Cover Goal Data`)) null 4.0))

(event `self.Initialize`
  (params (OwnerActor :type "Actor Object Reference") (owner :type "BehaviourSelectorComponent Object Reference"))
  (bind _asshooter_base_character (cast `ShooterBaseCharacter` OwnerActor))
  (set `self.Owner Actor` _asshooter_base_character))

(fn `GetSelectionScore`
  (params (GoalData :type "BaseGoalData Object Reference"))
  (returns (ReturnValue :type "Float (single-precision)"))
  (return 1.0))