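; Utility AI behaviour that makes a ShooterBaseCharacter reload its weapon.
; It is eligible whenever the clip is not full, and its selection score is zero until ammo runs low, then rises in two tiers as the clip empties.
; On enter it triggers the reload and stays non-interruptible for the weapon's reload time before completing, or fails if the owner is not a shooter character.
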(event `self.Initialize`
  (params (OwnerActor :type "Actor Object Reference") (owner :type "BehaviourSelectorComponent Object Reference"))
  (set `self.Owner Actor` OwnerActor))

(event `self.BehaviourEnter`
  (params (GoalData :type "BaseGoalData Object Reference"))
  (set `self.M_BehaviourState` "RUNNING")
  (set `self.M_BehaviourInterruptibilityState` "NOTINTERRUPTIBLE")
  (bind _asshooter_base_character (cast `ShooterBaseCharacter` (`self.Owner Actor`))
    (:`then`
      (`WeaponInterface.ReloadWeapon` _asshooter_base_character)
      (bind _returnvalue (`WeaponInterface.GetWeaponProperties` _asshooter_base_character))
      (`KismetSystemLibrary.Delay` (`WeaponProperties.WeaponReloadTime` _returnvalue))
      (set `self.M_BehaviourState` "COMPLETED")
      (set `self.M_BehaviourInterruptibilityState` "INTERRUPTIBLE"))
    (:`CastFailed`
      (set `self.M_BehaviourState` "FAILED"))))

(event `self.BehaviourExit`)

(fn `CheckPreConditions`
  (params (GoalData :type "BaseGoalData Object Reference"))
  (returns (ReturnValue :type Boolean))
  (bind _asshooter_base_character (cast `ShooterBaseCharacter` (`self.Owner Actor`))
    (:`then`
      (bind _returnvalue (`WeaponInterface.GetPercentAmmoLeftInClip` _asshooter_base_character))
      (return (!= _returnvalue 100.0)))
    (:`CastFailed`
      (return false))))

(fn `GetSelectionScore`
  (params (GoalData :type "BaseGoalData Object Reference"))
  (returns (ReturnValue :type "Float (single-precision)"))
  (bind _asshooter_base_character (cast `ShooterBaseCharacter` (`self.Owner Actor`)))
  (bind _returnvalue (message `WeaponInterface.GetPercentAmmoLeftInClip` _asshooter_base_character))
  (if (<= _returnvalue 30.0)
    (if (<= _returnvalue 15.0)
      (return 20.0)
      (else
        (return 15.0)))
    (else
      (return 0.0))))