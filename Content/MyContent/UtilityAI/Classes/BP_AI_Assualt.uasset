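; BP_AI_Assualt is an AI actor Blueprint, apparently the assault variant in a UtilityAI setup, that adds a camera-facing text label.
; Each Tick runs the parent logic, then turns the Text component toward the player camera manager's location with a look-at rotation, creating a billboard effect.
; The construction script only calls its parent, and no utility scoring or assault behavior appears in these graphs.
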(event `self.ReceiveTick`
  (params (DeltaSeconds :type "Float (single-precision)"))
  (bind _text (`self.Text`))
  (`parent.ReceiveTick` DeltaSeconds)
  (`SceneComponent.K2_SetWorldRotation` _text (`KismetMathLibrary.FindLookAtRotation` (`SceneComponent.K2_GetComponentLocation` _text) (`SceneComponent.K2_GetComponentLocation` (`Actor.RootComponent` (`GameplayStatics.GetPlayerCameraManager` 0)))) false false))

(fn `UserConstructionScript`
  (`parent.UserConstructionScript`))