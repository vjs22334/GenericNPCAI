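; Player character Blueprint for a shooter that keeps the on-screen ammo count in sync with the character's clip.
; Every Tick it reads the ammo in the clip, casts the first player controller's HUD to ShooterHUD and passes the value to its HudRef for display.
; The update is polled each frame, and the Blueprint adds no other active logic beyond calling the parent construction script.
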(event `self.ReceiveTick`
  (params (DeltaSeconds :type "Float (single-precision)"))
  (bind _returnvalue (`WeaponInterface.GetAmmoInClip`))
  (bind _asshooter_hud (cast `/Game/MyContent/Widget/ShooterHUD` (`PlayerController.GetHUD` (`GameplayStatics.GetPlayerController` 0))))
  (`/Game/MyContent/Widget/WB_PlayerHUD.UpdateAmmoCount` (`/Game/MyContent/Widget/ShooterHUD.HudRef` _asshooter_hud) (`KismetMathLibrary.Conv_IntToInt64` _returnvalue)))

(fn `UserConstructionScript`
  (`parent.UserConstructionScript`))