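; BP_Shooter_AI_Character is an AI shooter character with team-based coloring and an overhead behaviour debug display.
; BeginPlay disables shadows on the health and debug widgets, links the debug widget to its component, and applies blue or red Manny materials from the Detection team.
; Tick pushes the BehaviourSelector's current behaviour name to the debug widget, showing "DEAD" once the selector is no longer valid.
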(event `self.ReceiveBeginPlay`
  (bind _behaviour_debug_widget (`self.Behaviour Debug Widget`))
  (bind _mesh (`self.Mesh`))
  (`parent.ReceiveBeginPlay`)
  (`PrimitiveComponent.SetCastShadow` (`self.HealthBarWidget`) false)
  (`PrimitiveComponent.SetCastShadow` _behaviour_debug_widget false)
  (bind _aswb_behaviour_debug (cast `/Game/MyContent/Widget/WB_BehaviourDebug` (`WidgetComponent.GetWidget` _behaviour_debug_widget)))
  (set `/Game/MyContent/Widget/WB_BehaviourDebug.AttachedSceneComponent` _behaviour_debug_widget _aswb_behaviour_debug)
  ;[1 1 1] Team Color
  (if (== (`DetectionComponent.MyTeam` (`self.Detection`)) 1)
    ;;[1 1 1] Team 1 (blue)
    (`PrimitiveComponent.SetMaterial` _mesh 0 "/Game/MyContent/Character/Mannequins/Materials/TeamColor/MI_Manny_00_Team_A.MI_Manny_00_Team_A")
    (`PrimitiveComponent.SetMaterial` _mesh 1 "/Game/MyContent/Character/Mannequins/Materials/TeamColor/MI_Manny_01_Team_A.MI_Manny_01_Team_A")
    (else
      ;;[1 1 1] Not Team 1 (red)
      (`PrimitiveComponent.SetMaterial` _mesh 0 "/Game/MyContent/Character/Mannequins/Materials/TeamColor/MI_Manny_00_Team_B.MI_Manny_00_Team_B")
      (`PrimitiveComponent.SetMaterial` _mesh 1 "/Game/MyContent/Character/Mannequins/Materials/TeamColor/MI_Manny_01_Team_B.MI_Manny_01_Team_B"))))

(event `self.ReceiveTick`
  (params (DeltaSeconds :type "Float (single-precision)"))
  (bind _behaviourselector (`self.BehaviourSelector`))
  (bind _returnvalue (`KismetSystemLibrary.IsValid` _behaviourselector))
  ;[1 1 1] Debug widget
  (if _returnvalue
    (bind _returnvalue_2 (`BehaviourSelectorComponent.GetCurrentBehaviourName` _behaviourselector)))
  (bind _aswb_behaviour_debug (cast `/Game/MyContent/Widget/WB_BehaviourDebug` (`WidgetComponent.GetWidget` (`self.Behaviour Debug Widget`))))
  (`/Game/MyContent/Widget/WB_BehaviourDebug.SetBehaviourName` _aswb_behaviour_debug (`KismetMathLibrary.SelectString` _returnvalue_2 "DEAD" _returnvalue)))

(fn `UserConstructionScript`
  (`parent.UserConstructionScript`))