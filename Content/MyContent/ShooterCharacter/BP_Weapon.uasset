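; BP_Weapon is a player-input weapon that provides automatic hitscan fire and reloading, tuned by WeaponData.
; Holding left mouse loops Fire with rate-of-fire delays; an empty magazine or R triggers a timed reload.
; Fire line-traces from the owner's location, consumes ammo and applies damage through HealthSystemInterface.
; The trace end omits the start-location offset, and the Reload function is an unused stub.
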(event `self.ReceiveTick`
  (params (DeltaSeconds :type "Float (single-precision)")))

(event `self.ReceiveBeginPlay`
  ;[1 1 1] Setting Ammo Count
  (bind _weapondata (`self.WeaponData`)
    (:`then`
      (set `self.CurrentAmmoInMag` (`WeaponProperties.WeaponAmmoCount` _weapondata)))
    (:`else`)))

(event `Key|LeftMouseButton`
  (params (Key :type "Key Structure"))
  ;[1 1 1] Pew Pew input
  (:`Pressed`
    (set `self.IsFiring?` true)
    ;[1 1 1] Firing Logic
    (if (`self.IsFiring?`) :!label _label
      (if (> (`self.CurrentAmmoInMag`) 0.0)
        (if (`self.CanFire?`)
          (set `self.CanFire?` false)
          (`self.Fire`)
          (bind _weapondata (`self.WeaponData`)
            (:`then`
              (`KismetSystemLibrary.Delay` (`WeaponProperties.WeaponRateOfFire` _weapondata))
              (set `self.CanFire?` true)
              (goto _label))
            (:`else`)))
        (elif (not (`self.Reloading`))
          ;[1 1 1] Reloading
          (bind _weapondata_2 (`self.WeaponData` :!label _label_2)
            (:`then`
              (bind _weaponreloadtime (`WeaponProperties.WeaponReloadTime` _weapondata_2))
              (`KismetSystemLibrary.PrintString` "Reloading" true true (struct :`G` 0.66 :`B` 1.0 :`A` 1.0) _weaponreloadtime)
              (set `self.Reloading` true)
              (`KismetSystemLibrary.Delay` _weaponreloadtime)
              (set `self.CurrentAmmoInMag` (`WeaponProperties.WeaponAmmoCount` _weapondata_2))
              (set `self.Reloading` false)
              (`KismetSystemLibrary.PrintString` "Reloaded" true true (struct :`R` 0.15214 :`G` 1.0 :`A` 1.0) 1.0))
            (:`else`))))))
  (:`Released`
    (set `self.IsFiring?` false)))

(event `Key|R`
  (params (Key :type "Key Structure"))
  (:`Pressed`
    (goto _label_2)))

(fn `Fire`
  (bind (_returnvalue_location _returnvalue_rotation) (`KismetMathLibrary.BreakTransform` (`Actor.GetTransform` (`self.GetOwner`))))
  (bind _weapondata (`self.WeaponData`)
    (:`then`
      (bind (_outhit _returnvalue) (`KismetSystemLibrary.LineTraceSingle` :`Start` _returnvalue_location :`End` (* (`KismetMathLibrary.GetForwardVector` _returnvalue_rotation) (* (`WeaponProperties.WeaponBulletRange` _weapondata) 100.0)) :`TraceChannel` "TraceTypeQuery4" :`DrawDebugType` "ForDuration" :`DrawTime` 1.0))
      (set `self.CurrentAmmoInMag` (- (`self.CurrentAmmoInMag`) 1.0))
      (bind (_bblockinghit _binitialoverlap _time _distance _location _impactpoint _normal _impactnormal _physmat _hitactor) (`GameplayStatics.BreakHitResult` _outhit))
      (if (and (`KismetSystemLibrary.DoesImplementInterface` _hitactor "/Script/AIPlayground.HealthSystemInterface") _returnvalue)
        (bind _ashealth_system_interface (cast `HealthSystemInterface` _hitactor))
        (`HealthSystemInterface.ApplyDamage` _ashealth_system_interface (`WeaponProperties.WeaponDamage` _weapondata))))
    (:`else`)))

(fn `Reload`
  (`KismetSystemLibrary.PrintString` "Reloading")
  (bind _weapondata (`self.WeaponData`)
    (:`then`)
    (:`else`)))