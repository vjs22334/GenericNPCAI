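; Grenade-throwing Blueprint for its owning shooter character, triggered by right mouse button or a ThrowGrenade event.
; BeginPlay caches the owner, and a throw starts the throw montage on its mesh, spawning A_Nade immediately at the GrenadeREF location without waiting for an animation notify.
; The grenade's sphere gets a physics velocity scaled by Force, directed from the character's location through the spawn point rather than along aim.
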(event `self.ReceiveBeginPlay`
  (bind _asbp_template_shooter_base_character (cast `/Game/MyContent/Blueprint/BP_Template_ShooterBaseCharacter` (`self.GetOwner`)))
  (set `self.Player Reference` _asbp_template_shooter_base_character))

(event `Key|RightMouseButton`
  (params (Key :type "Key Structure"))
  (bind _player_reference (`self.Player Reference`))
  (:`Pressed`
    (`|PlayMontage` (`Character.Mesh` _player_reference) "/Game/MyContent/Animation/Anims/nadethrow_Montage.nadethrow_Montage" :!label _label
      (:`then`
        (bind _returnvalue (`|SpawnActorFromClass` "/Game/MyContent/Blueprint/A_Nade.A_Nade_C" (`KismetMathLibrary.MakeTransform` (`SceneComponent.K2_GetComponentLocation` (`/Game/MyContent/Blueprint/BP_Template_ShooterBaseCharacter.Grenade REF` _player_reference)) (`KismetMathLibrary.Conv_VectorToRotator` (`KismetMathLibrary.GetForwardVector` (`Actor.K2_GetActorRotation` _player_reference)))) "Undefined" "OverrideRootScale" null null))
        (`PrimitiveComponent.SetPhysicsLinearVelocity` (`/Game/MyContent/Blueprint/A_Nade.Sphere` _returnvalue) (* (`KismetMathLibrary.GetDirectionUnitVector` (`Actor.K2_GetActorLocation` (`self.Player Reference`)) (`Actor.K2_GetActorLocation` _returnvalue)) (`self.Force`)) false "None")))))

(event `self.ThrowGrenade`
  (goto _label))