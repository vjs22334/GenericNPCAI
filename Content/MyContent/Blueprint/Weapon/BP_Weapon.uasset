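; BP_Weapon runs an automatic, data-driven weapon for its owning shooter character, using that character's Weapon skeletal mesh.
; WeaponData supplies mesh, magazine size, damage, fire rate and reload time.
; Left mouse or FireWeapon starts a Delay-gated loop spawning BP_Projectile from the Muzzle socket.
; An empty magazine or R triggers a timed reload in the event graph; the separate Reload function is a stub.
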(event `self.SetupWeapon`
  ;[1 1 1] Setup on Begin Play
  (bind _weapondata (`self.WeaponData`)
    (:`then`
      (set `self.CurrentAmmoInMag` (`WeaponProperties.WeaponAmmoCount` _weapondata))
      (`SkeletalMeshComponent.SetSkeletalMeshAsset` (`self.Weapon Skeleton Mesh Reference`) (`WeaponProperties.WeaponMesh` _weapondata)))
    (:`else`)))

(event `self.ReceiveBeginPlay`
  ;[1 1 1] Setting Default Values & Variables
  (set `self.CanFire?` true)
  (bind _asbp_template_shooter_base_character (cast `/Game/MyContent/Blueprint/BP_Template_ShooterBaseCharacter` (`self.GetOwner`)))
  (bind _output_get (set `self.Player Reference` _asbp_template_shooter_base_character))
  (set `self.Weapon Skeleton Mesh Reference` (`/Game/MyContent/Blueprint/BP_Template_ShooterBaseCharacter.Weapon` _output_get)))

(event `self.FireWeapon`
  ;[1 1 1] Pew Pew input
  (set `self.IsFiring?` true :!label _label)
  ;[1 1 1] Firing Logic
  (if (`self.IsFiring?`) :!label _label_2
    (if (> (`self.CurrentAmmoInMag`) 0.0)
      (if (`self.CanFire?`)
        (set `self.CanFire?` false)
        (`self.Fire`)
        (bind _weapondata (`self.WeaponData`)
          (:`then`
            (`KismetSystemLibrary.Delay` (`WeaponProperties.WeaponRateOfFire` _weapondata))
            (set `self.CanFire?` true)
            (goto _label_2))
          (:`else`)))
      (elif (not (`self.Reloading`))
        ;[1 1 1] Reloading
        (bind _weapondata_2 (`self.WeaponData` :!label _label_3)
          (:`then`
            (bind _weaponreloadtime (`WeaponProperties.WeaponReloadTime` _weapondata_2))
            (`KismetSystemLibrary.PrintString` "Reloading" true true (struct :`G` 0.66 :`B` 1.0 :`A` 1.0) _weaponreloadtime)
            (set `self.Reloading` true)
            (`KismetSystemLibrary.Delay` _weaponreloadtime)
            (set `self.CurrentAmmoInMag` (`WeaponProperties.WeaponAmmoCount` _weapondata_2))
            (set `self.Reloading` false)
            (`KismetSystemLibrary.PrintString` "Reloaded" true true (struct :`R` 0.15214 :`G` 1.0 :`A` 1.0) 1.0))
          (:`else`))))))

(event `Key|LeftMouseButton`
  (params (Key :type "Key Structure"))
  ;[1 1 1] Pew Pew input
  (:`Pressed`
    (goto _label))
  (:`Released`
    (set `self.IsFiring?` false)))

(event `Key|R`
  (params (Key :type "Key Structure"))
  (:`Pressed`
    (goto _label_3)))

(fn `Fire`
  (bind (_returnvalue_location _returnvalue_rotation) (`KismetMathLibrary.BreakTransform` (`SceneComponent.GetSocketTransform` (`/Game/MyContent/Blueprint/BP_Template_ShooterBaseCharacter.Weapon` (`self.Player Reference`)) "Muzzle" "RTS_World")))
  (bind _returnvalue (`|SpawnActorFromClass` "/Game/MyContent/Blueprint/BP_Projectile.BP_Projectile_C" (`KismetMathLibrary.MakeTransform` _returnvalue_location (`KismetMathLibrary.Conv_VectorToRotator` (`KismetMathLibrary.GetForwardVector` _returnvalue_rotation))) "Undefined" "OverrideRootScale" null null))
  (bind _weapondata (`self.WeaponData`)
    (:`then`
      (set `/Game/MyContent/Blueprint/BP_Projectile.Damage` (`WeaponProperties.WeaponDamage` _weapondata) _returnvalue)
      (set `self.CurrentAmmoInMag` (- (`self.CurrentAmmoInMag`) 1.0)))
    (:`else`)))

(fn `Reload`
  (`KismetSystemLibrary.PrintString` "Reloading")
  (bind _weapondata (`self.WeaponData`)
    (:`then`)
    (:`else`)))