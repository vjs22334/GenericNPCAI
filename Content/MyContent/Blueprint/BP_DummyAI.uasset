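; BP_DummyAI is a simple test AI that repeatedly repositions itself using the EQS_Strafe query, without a Behavior Tree in this graph.
; A DoOnce on Tick stores the player character as Target, runs the query and moves to the resulting location.
; Only a successful move re-arms the DoOnce after a delay, so a failed move stalls the loop.
; A team-based DetectionSystem lookup is left unconnected.
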(event `self.ReceiveBeginPlay`
  (`parent.ReceiveBeginPlay`))

(event `self.ReceiveTick`
  (params (DeltaSeconds :type "Float (single-precision)"))
  (`/Engine/EditorBlueprintResources/StandardMacros.DoOnce` false :!label _label
    (:`Completed`
      (bind _asbp_shooter_player_character (cast `/Game/MyContent/Blueprint/BP_Shooter_Player_Character` (`GameplayStatics.GetPlayerPawn` 0)))
      (set `self.Target` _asbp_shooter_player_character)
      ;[1 1 1] Run EQS and Move To
      (bind _returnvalue (`EnvQueryManager.RunEQSQuery` "/Game/MyContent/EQS/EQS_Strafe.EQS_Strafe" self "SingleResult"))
      (`/Engine/EditorBlueprintResources/StandardMacros.IsValid` _returnvalue
        (:`Is Valid`
          (add `EnvQueryInstanceBlueprintWrapper.OnQueryFinishedEvent` _returnvalue (delegate `CustomEvent`)))))))

(event `CustomEvent`
  (params (QueryInstance :type "EnvQueryInstanceBlueprintWrapper Object Reference") (QueryStatus :type "EEnvQueryStatus Enum" :default "Processing"))
  ;[1 1 1] Run EQS and Move To
  (bind _resultlocations (`EnvQueryInstanceBlueprintWrapper.GetQueryResultsAsLocations` QueryInstance))
  (`|AIMoveTo` self (`|GetArrayItem` _resultlocations) null
    (:`OnSuccess`
      (`KismetSystemLibrary.Delay` 4.0)
      (goto _label :!via `Reset`))))

(fn `UserConstructionScript`
  (`parent.UserConstructionScript`))