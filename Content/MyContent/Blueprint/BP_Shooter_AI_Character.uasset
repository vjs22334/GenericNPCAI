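; BP_Shooter_AI_Character is an AI character Blueprint that shows the name of its current behaviour on an attached debug widget.
; On BeginPlay it passes the BehaviourDebugWidget component to its WB_BehaviourDebug widget as the attached scene component.
; Every Tick it polls BehaviourSelector for the current behaviour name and pushes it to that widget.
; The construction script only calls the parent, and no behaviour logic is defined in these graphs.
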(event `self.ReceiveBeginPlay`
  (bind _behaviour_debug_widget (`self.Behaviour Debug Widget`))
  (`parent.ReceiveBeginPlay`)
  (bind _aswb_behaviour_debug (cast `/Game/MyContent/Blueprint/Widget/WB_BehaviourDebug` (`WidgetComponent.GetWidget` _behaviour_debug_widget)))
  (set `/Game/MyContent/Blueprint/Widget/WB_BehaviourDebug.AttachedSceneComponent` _behaviour_debug_widget _aswb_behaviour_debug))

(event `self.ReceiveTick`
  (params (DeltaSeconds :type "Float (single-precision)"))
  (bind _returnvalue (`BehaviourSelectorComponent.GetCurrentBehaviourName` (`self.BehaviourSelector`)))
  (bind _aswb_behaviour_debug (cast `/Game/MyContent/Blueprint/Widget/WB_BehaviourDebug` (`WidgetComponent.GetWidget` (`self.Behaviour Debug Widget`))))
  (`/Game/MyContent/Blueprint/Widget/WB_BehaviourDebug.SetBehaviourName` _aswb_behaviour_debug _returnvalue))

(fn `UserConstructionScript`
  (`parent.UserConstructionScript`))