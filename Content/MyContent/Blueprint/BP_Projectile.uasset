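; Projectile actor that damages pawns it overlaps and then destroys itself.
; Each Tick it runs a box overlap query sized to its Box component, filtered to pawns, instead of relying on overlap events.
; Pawns implementing HealthSystemInterface receive its Damage through that interface, and a damage event crediting the Shooter is reported, presumably for AI damage sensing.
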(event `self.ReceiveTick`
  (params (DeltaSeconds :type "Float (single-precision)"))
  (bind _returnvalue (`self.K2_GetActorLocation`))
  (bind _damage (`self.Damage`))
  (bind _outactors (`KismetSystemLibrary.BoxOverlapActors` _returnvalue (`BoxComponent.GetScaledBoxExtent` (`self.Box`)) (`|MakeArray` "ObjectTypeQuery3" :!type "EObjectTypeQuery Enum") "/Script/Engine.Pawn" (`|MakeArray` self :!type "Actor Object Reference")))
  (for _array_element _outactors
    (bind _ashealth_system_interface (cast `HealthSystemInterface` _array_element))
    (`HealthSystemInterface.ApplyDamage` _ashealth_system_interface _damage)
    (`AISense_Damage.ReportDamageEvent` _array_element (`self.Shooter`) _damage _returnvalue)
    (`self.K2_DestroyActor`)))

(fn `UserConstructionScript`)